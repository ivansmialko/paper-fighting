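; Player character Blueprint for the Businessman, a flipbook-sprite character that overrides the attack event to allow only ground attacks.
; When not falling, a DoOnce gate stops movement, clears blocking and calls GroundAttackPlayer.
; After a delay based on the current flipbook's length, it restores the max walk speed, prints a debug string and reopens the gate.
; The other events are disabled stubs, and construction only calls the parent.
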(event `self.AttackPlayer`
  ;[1 1 1] Allow only ground attacks
  (if (not (`NavMovementComponent.IsFalling` (`self.CharacterMovement`)))
    (`/Engine/EditorBlueprintResources/StandardMacros.DoOnce` false :!label _label
      (:`Completed`
        (set `CharacterMovementComponent.MaxWalkSpeed` 0.0 (`self.CharacterMovement`))
        (set `self.IsBlocking` false)
        (`self.GroundAttackPlayer`)
        (`KismetSystemLibrary.Delay` (- (`PaperFlipbookComponent.GetFlipbookLength` (`self.Sprite`)) 0.0))
        (set `CharacterMovementComponent.MaxWalkSpeed` (`self.PlayerMaxSpeed`) (`self.CharacterMovement`))
        (`KismetSystemLibrary.PrintString` "Reset")
        (goto _label :!via `Reset`)))))

(fn `UserConstructionScript`
  (`parent.UserConstructionScript`))